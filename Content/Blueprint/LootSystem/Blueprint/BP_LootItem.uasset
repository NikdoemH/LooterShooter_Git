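; BP_LootItem is a loot drop actor that pops out on spawn and shows its stats in a widget when looked at.
; The construction script picks the sphere's material from the item's rarity.
; On BeginPlay a randomized upward impulse launches the sphere; after a delay physics stops, collision becomes query-only, and the widget moves above it and receives score and weapon stats.
; Look events toggle widget visibility, resetting its world rotation when shown.
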(event Custom|LookAtItem
  (bind _loot_widget (Variables|Default|GetLoot_Widget))
  (Rendering|SetVisibility _loot_widget true false)
  (Transformation|SetWorldRotation _loot_widget "0, 0, 0" false false))

(event Custom|StopLookingAtItem
  (Rendering|SetVisibility (Variables|Default|GetLoot_Widget) false false))

(event EventBeginPlay
  (bind _itemdetals (Variables|Default|GetItemDetals))
  (bind _sphere (Variables|Default|GetSphere))
  (bind _sphere_2 (Variables|Default|GetSphere))
  (bind (_rarity _lootscore _itemstats) (Utilities|Struct|BreakRarity_Struct _itemdetals))
  (bind _returnvalue (Transformation|GetWorldLocation _sphere_2))
  (bind (_shootspeed _dmg _ammosize) (Utilities|Struct|BreakStat_Struct _itemstats))
  (Physics|AddImpulse (Variables|Default|GetSphere) (* (Math|Vector|MakeVector (Math|Random|RandomFloatinRange -1.0 1.0) (Math|Random|RandomFloatinRange -1.0 1.0) 1.0) (Variables|Default|GetImpulsePower)) "None" true)
  (Utilities|FlowControl|Delay 3.5)
  (Physics|SetSimulatePhysics _sphere false)
  (Collision|SetCollisionEnabled _sphere "QueryOnly")
  (Transformation|SetWorldLocation (Variables|Default|GetLoot_Widget) (Math|Vector|MakeVector (.x _returnvalue) (.y _returnvalue) (+ (.z _returnvalue) 25.0)) false false)
  (bind _aswg_loot_widget (Utilities|Casting|CastToWG_LootWidget (UserInterface|GetUserWidgetObject (Variables|Default|GetLoot_Widget))))
  (Variables|/Game/Widget/UI/WG_LootWidget.WG_LootWidget_C|SetLootScore _aswg_loot_widget _lootscore)
  (Variables|/Game/Widget/UI/WG_LootWidget.WG_LootWidget_C|SetShootSpeed _aswg_loot_widget _shootspeed)
  (Variables|/Game/Widget/UI/WG_LootWidget.WG_LootWidget_C|SetDMG _aswg_loot_widget _dmg)
  (Variables|/Game/Widget/UI/WG_LootWidget.WG_LootWidget_C|SetAmmoSize _aswg_loot_widget _ammosize))

(fn ConstructionScript
  (Rendering|Material|SetMaterial (Variables|Default|GetSphere) 0 (Utilities|Select :Index (.Rarity (Utilities|Struct|BreakRarity_Struct (Variables|Default|GetItemDetals))) :NewEnumerator6 "/Game/LevelPrototyping/Materials/MI_Solid_Blue.MI_Solid_Blue" :NewEnumerator0 "/Game/Blueprint/LootSystem/Material/MI_CommonItem.MI_CommonItem" :NewEnumerator1 "/Game/Blueprint/LootSystem/Material/MI_UnCommonItem.MI_UnCommonItem" :NewEnumerator2 "/Game/Blueprint/LootSystem/Material/Mi_RareItem.Mi_RareItem" :NewEnumerator3 "/Game/Blueprint/LootSystem/Material/Mi_EpickItem.Mi_EpickItem" :NewEnumerator4 "/Game/Blueprint/LootSystem/Material/Mi_Legendary.Mi_Legendary" :NewEnumerator5 "/Game/Blueprint/LootSystem/Material/Mi_GodlyIItem.Mi_GodlyIItem")))