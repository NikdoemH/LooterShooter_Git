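; BP_LootSpawner is an actor that spawns a BP_LootItem at its own location every second on a looping timer.
; ChooseRarity makes a weighted random roll over the Rarity map stored in the BP_LootInstance game instance.
; GenerateLootScore scales a random base score by a per-rarity multiplier.
; Each spawned item receives the rarity and rounded score as a struct.
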(event Custom|CreateLoot
  (bind _rarity (CallFunction|ChooseRarity))
  (bind _returnvalue (CallFunction|GenerateLootScore _rarity))
  (Game|SpawnActorfromClass "/Game/Blueprint/LootSystem/Blueprint/BP_LootItem.BP_LootItem_C" (Math|Conversions|ToTransform(Vector) (Transformation|GetActorLocation)) "Undefined" "MultiplyWithRoot" 0 (Utilities|Struct|MakeRarity_Struct _rarity _returnvalue) 0))

(event EventBeginPlay
  (Utilities|Time|SetTimerbyEvent (delegate Custom|CreateLoot) 1.0 true))

(fn ConstructionScript)

(fn ChooseRarity
  (bind _asbp_loot_instance (Utilities|Casting|CastToBP_LootInstance (Game|GetGameInstance)))
  (bind _keys (Utilities|Map|Keys (Variables|/Game/Blueprint/LootSystem/Blueprint/BP_LootInstance.BP_LootInstance_C|GetRarity _asbp_loot_instance)))
  (for _array_element _keys
    (LocalVariables|SetSumOfRarity (+ (.Value (Utilities|Map|Find (Variables|/Game/Blueprint/LootSystem/Blueprint/BP_LootInstance.BP_LootInstance_C|GetRarity _asbp_loot_instance) _array_element)) (LocalVariables|GetSumOfRarity))))
  (LocalVariables|SetLootRoll (Math|Random|RandomFloatinRange 0.0 (LocalVariables|GetSumOfRarity)))
  (bind _keys_2 (Utilities|Map|Keys (Variables|/Game/Blueprint/LootSystem/Blueprint/BP_LootInstance.BP_LootInstance_C|GetRarity _asbp_loot_instance)))
  (bind _array_element_2 (Utilities|Array|ForEachLoopwithBreak _keys_2 :!label _label)
    (:LoopBody
      (if (>= (.Value (Utilities|Map|Find (Variables|/Game/Blueprint/LootSystem/Blueprint/BP_LootInstance.BP_LootInstance_C|GetRarity _asbp_loot_instance) _array_element_2)) (LocalVariables|GetLootRoll))
        (LocalVariables|SetRarityOut _array_element_2)
        (goto _label Break)
        (else
          (LocalVariables|SetLootRoll (- (LocalVariables|GetLootRoll) (.Value (Utilities|Map|Find (Variables|/Game/Blueprint/LootSystem/Blueprint/BP_LootInstance.BP_LootInstance_C|GetRarity _asbp_loot_instance) _array_element_2)))))))
    (:Completed
      (return (LocalVariables|GetRarityOut)))))

(fn GenerateLootScore
  (params (Rarity :type Rarity_ENUM%20Enum :default "NewEnumerator6"))
  (LocalVariables|SetLootScoreMultiplier (Utilities|Select :Index Rarity :NewEnumerator6 0.0 :NewEnumerator0 0.1 :NewEnumerator1 1.0 :NewEnumerator2 5.0 :NewEnumerator3 1e+01 :NewEnumerator4 2e+01 :NewEnumerator5 5e+01))
  (LocalVariables|SetPreMultiplierScore (Math|Random|RandomFloatinRange 5e+01 2e+02))
  (return (Math|Float|Round (* (LocalVariables|GetPreMultiplierScore) (LocalVariables|GetLootScoreMultiplier)))))